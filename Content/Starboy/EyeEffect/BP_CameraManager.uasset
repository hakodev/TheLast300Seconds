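; BP_CameraManager is a debug-style camera switcher that toggles between a first-person camera and a sequence camera.
; Pressing Q drives a FlipFlop that alternately activates the root component of FPCam or SeqCam and deactivates the other.
; It only sets component active states, with no explicit view target change or blend, and its construction script is empty.
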(event Input|KeyboardEvents|Q
  (params (Key :type Key%20Structure :default "None"))
  (:Pressed
    (Utilities|FlowControl|FlipFlop
      (:A
        (Components|Activation|SetActive (Variables|/Script/Engine.Actor|GetRootComponent (Variables|Default|GetFPCam)) true false)
        (Components|Activation|SetActive (Variables|/Script/Engine.Actor|GetRootComponent (Variables|Default|GetSeqCam)) false false))
      (:B
        (Components|Activation|SetActive (Variables|/Script/Engine.Actor|GetRootComponent (Variables|Default|GetFPCam)) false false)
        (Components|Activation|SetActive (Variables|/Script/Engine.Actor|GetRootComponent (Variables|Default|GetSeqCam)) true false)))))

(fn ConstructionScript)