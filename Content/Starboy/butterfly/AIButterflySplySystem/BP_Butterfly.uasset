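; BP_Butterfly is a butterfly in the AI butterfly system that detects player contact and exposes a path.
; Its Box overlap events set PlayerTouch when BP_ThirdPersonCharacter enters or leaves, and print the value as debug output.
; PathFly returns the Path variable, while the flag is not read for any behavior here and no movement logic is present.
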(event OnComponentBeginOverlap(Box)
  (params (OverlappedComponent :type Primitive%20Component%20Object%20Reference) (OtherActor :type Actor%20Object%20Reference) (OtherComp :type Primitive%20Component%20Object%20Reference) (OtherBodyIndex :type Integer) (bFromSweep :type Boolean) (SweepResult :type Hit%20Result%20Structure%20%28by%20ref%29))
  (Utilities|Casting|CastToBP_ThirdPersonCharacter OtherActor)
  (bind _output_get (Variables|Default|SetPlayerTouch true))
  (Development|PrintString (Utilities|String|ToString(Boolean) _output_get) true true "(R=1.000000,G=1.000000,B=1.000000,A=1.000000)"))

(event OnComponentEndOverlap(Box)
  (params (OverlappedComponent :type Primitive%20Component%20Object%20Reference) (OtherActor :type Actor%20Object%20Reference) (OtherComp :type Primitive%20Component%20Object%20Reference) (OtherBodyIndex :type Integer))
  (Utilities|Casting|CastToBP_ThirdPersonCharacter OtherActor)
  (bind _output_get (Variables|Default|SetPlayerTouch false))
  (Development|PrintString (Utilities|String|ToString(Boolean) _output_get) true true "(R=1.000000,G=1.000000,B=1.000000,A=1.000000)"))

(fn ConstructionScript)

(fn PathFly
  (return (Variables|Default|GetPath)))