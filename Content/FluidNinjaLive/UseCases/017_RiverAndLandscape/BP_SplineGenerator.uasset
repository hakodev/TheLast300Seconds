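; Spline-driven river generator that builds a chain of spline meshes tagged "River" along its spline.
; The construction script splits the spline into sections sized from actor scale and a size adjustment, clamps tangents to section length, and applies a placeholder mesh and optional material.
; On BeginPlay it swaps in the high-detail in-game mesh, if set, and enables collision that blocks Camera and Visibility.
; Character swimming calls are present but disconnected.
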(event EventBeginPlay
  (Utilities|IsValid (Variables|SplineGenerator|GetIn-gameHighdetailStaticmesh)
    (:Is%20Valid
      (for _array_element (Actor|GetComponentsByClass self "/Script/Engine.SplineMeshComponent")
        (Components|StaticMesh|SetStaticMesh _array_element (Variables|SplineGenerator|GetIn-gameHighdetailStaticmesh))
        (Variables|/Script/Engine.ActorComponent|SetComponentTags _array_element (Utilities|Array|MakeArray "River"))
        (Collision|SetCollisionEnabled _array_element "QueryAndPhysics")
        (Collision|SetCollisionResponsetoChannel _array_element "ECC_Camera" "ECR_Block")
        (Collision|SetCollisionResponsetoChannel _array_element "ECC_Visibility" "ECR_Block")))
    (:Is%20Not%20Valid
      (Variables|SplineGenerator|SetIn-gameHighdetailStaticmesh (Variables|SplineGenerator|GetEditorPlaceholderStaticmesh)))))

(event Collision|EventActorBeginOverlap
  (params (OtherActor :type Actor%20Object%20Reference)))

(event EventTick
  (params (DeltaSeconds :type Float%20%28single-precision%29)))

(event Collision|EventActorEndOverlap
  (params (OtherActor :type Actor%20Object%20Reference)))

(fn ConstructionScript
  (bind _returnvalue (Transformation|GetActorScale3D))
  (bind _editorplaceholdermaterial (Variables|SplineGenerator|GetEditorPlaceholderMaterial))
  (bind _spline (Variables|Default|GetSpline))
  (Variables|SplineGenerator|SetSectionLength (* (Utilities|Select :Index (Variables|SplineGenerator|GetIn%20Forward%20Axis) :X (.x _returnvalue) :Y (.y _returnvalue) :Z (.z _returnvalue)) (* (Variables|SplineGenerator|GetSizeAdjutment) 1e+02)))
  (for _index (range 0 (- (Math|Float|Truncate (/ (Spline|GetSplineLength (Variables|Default|GetSpline)) (Variables|SplineGenerator|GetSectionLength))) 1))
    (bind _returnvalue_2 (AddComponent|AddSplineMeshComponent false))
    (Variables|/Script/Engine.ActorComponent|SetComponentTags _returnvalue_2 (Utilities|Array|MakeArray "River"))
    (SplineMesh|SetForwardAxis _returnvalue_2 (Variables|SplineGenerator|GetIn%20Forward%20Axis) true)
    (SplineMesh|SetStartandEnd _returnvalue_2 (Spline|GetLocationatDistanceAlongSpline _spline (* _index (Variables|SplineGenerator|GetSectionLength)) "Local") (Math|Vector|ClampVectorSize (Spline|GetTangentatDistanceAlongSpline _spline (* _index (Variables|SplineGenerator|GetSectionLength)) "Local") 0.0 (Variables|SplineGenerator|GetSectionLength)) (Spline|GetLocationatDistanceAlongSpline _spline (* (+ _index 1) (Variables|SplineGenerator|GetSectionLength)) "Local") (Math|Vector|ClampVectorSize (Spline|GetTangentatDistanceAlongSpline _spline (* (+ _index 1) (Variables|SplineGenerator|GetSectionLength)) "Local") 0.0 (Variables|SplineGenerator|GetSectionLength)) true :!class /Script/Engine.SplineMeshComponent)
    (Components|StaticMesh|SetStaticMesh _returnvalue_2 (Variables|SplineGenerator|GetEditorPlaceholderStaticmesh))
    (Utilities|IsValid _editorplaceholdermaterial
      (:Is%20Valid
        (Rendering|Material|SetMaterial _returnvalue_2 0 _editorplaceholdermaterial)))))