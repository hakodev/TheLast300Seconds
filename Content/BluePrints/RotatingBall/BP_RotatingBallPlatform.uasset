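; Rotating ball platform actor for a puzzle, with a lantern spiral that spins steadily on Tick.
; BeginPlay hides the linked puzzle cone and, if present, the puzzle camera.
; Disconnected logic would check the Face, Mosaic or Body puzzle, swap the sphere to a crystal material, reveal the cone and play a one-time camera cutaway.
; An all-solved finale camera sequence is also disconnected, so no completion response runs.
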(event EventBeginPlay
  (Rendering|SetActorHiddenInGame (Variables|Default|GetPuzzle%20Cone) true)
  (if (== (Variables|Default|GetPuzzle%20hasCam) true)
    (Rendering|SetActorHiddenInGame (Variables|Default|GetPuzzle%20Cam) true)))

(event EventTick
  (params (DeltaSeconds :type Float%20%28single-precision%29))
  (Transformation|AddLocalRotation (Variables|Default|GetlanternSprial) (Math|Rotator|MakeRotator 0.0 (* DeltaSeconds 3e+01) 0.0) false false))

(fn ConstructionScript)