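; BP_DynamicLevelMusic controls layered level music built on the MSS_DynamicLevelMusic sound, which it spawns as 2D audio on BeginPlay and immediately stops.
; PlayMusic starts playback, and StopMusic halts it, with a logarithmic fade-out unless NoFadeOut is set.
; AddMusicLayer increments the active layer and, within the MusicLayers count, uses a timeline to fade in that layer's float parameter, named from a prefix plus the index.
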(event Custom|PlayMusic
  (Audio|Components|Audio|Play (Variables|Default|GetSoundPlayer) 0.0))

(event Custom|StopMusic
  (params (NoFadeOut :type Boolean))
  (bind _soundplayer (Variables|Default|GetSoundPlayer))
  (bind _fadeduration (Variables|Default|GetFadeDuration))
  (if NoFadeOut
    _
    (else
      (Audio|Components|Audio|AdjustVolume _soundplayer _fadeduration 0.0 "Logarithmic" :!class /Script/Engine.AudioComponent)
      (Utilities|FlowControl|Delay _fadeduration)))
  (Audio|Components|Audio|Stop _soundplayer))

(event Custom|AddMusicLayer
  (bind _result (Math|Integer|IncrementInt (Variables|Default|GetActiveMusicLayer))
    (:%20%20
      (bind _output_get (Variables|Default|SetActiveMusicLayer _result))
      (if (<= _output_get (Utilities|Array|Length (Variables|Default|GetMusicLayers)))
        (bind _fadeamount (Timeline|FadeIn PlayFromStart)
          (:Update
            (Audio|Parameter|SetFloatParameter (Variables|Default|GetSoundPlayer) (Utilities|String|StringToName (Utilities|String|Append (Variables|Default|GetMusicLayerPrefix) (Utilities|String|ToString(Integer) (Variables|Default|GetActiveMusicLayer)))) _fadeamount :!class /Script/AudioExtensions.AudioParameterControllerInterface)))))))

(event EventBeginPlay
  (bind _returnvalue (Audio|SpawnSound2D "/Game/Audio/MSS_DynamicLevelMusic.MSS_DynamicLevelMusic" (Variables|Default|GetMusicVolumeMultiplier) 1.0 0.0 0 false false))
  (bind _output_get (Variables|Default|SetSoundPlayer _returnvalue))
  (Audio|Components|Audio|Stop _output_get))

(fn ConstructionScript)