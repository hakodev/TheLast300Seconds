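; BP_Guide is a timed "let go" puzzle trigger that shows a ninja actor while the third-person character stands in its collision box.
; Entering starts watching, stamps LastInputTime and lowers a point light; leaving stops it and restores the light.
; Tick polls elapsed time; after seven seconds it marks the top puzzle finished, swaps brain fire effects for heart visuals, and once adds music layers with a confirm sound.
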(event OnComponentBeginOverlap(CollisionBox)
  (params (OverlappedComponent :type Primitive%20Component%20Object%20Reference) (OtherActor :type Actor%20Object%20Reference) (OtherComp :type Primitive%20Component%20Object%20Reference) (OtherBodyIndex :type Integer) (bFromSweep :type Boolean) (SweepResult :type Hit%20Result%20Structure%20%28by%20ref%29))
  (Utilities|Casting|CastToBP_ThirdPersonCharacter OtherActor)
  (Variables|InputAndCollision|SetbWatchingActive true)
  (Input|EnableInput (Game|GetPlayerController 0))
  (Variables|InputAndCollision|SetLastInputTime (Utilities|Time|GetGameTimeinSeconds))
  (Rendering|Components|Light|SetIntensity (Variables|/Script/Engine.PointLight|GetPointLightComponent (Variables|Default|GetPointLightRef)) 7.5))

(event OnComponentEndOverlap(CollisionBox)
  (params (OverlappedComponent :type Primitive%20Component%20Object%20Reference) (OtherActor :type Actor%20Object%20Reference) (OtherComp :type Primitive%20Component%20Object%20Reference) (OtherBodyIndex :type Integer))
  (Utilities|Casting|CastToBP_ThirdPersonCharacter OtherActor)
  (Variables|InputAndCollision|SetbWatchingActive false)
  (Rendering|Components|Light|SetIntensity (Variables|/Script/Engine.PointLight|GetPointLightComponent (Variables|Default|GetPointLightRef)) 17.049931))

(event EventBeginPlay
  (Rendering|SetActorHiddenInGame (Variables|InputAndCollision|GetLetGoNinjaActor) true)
  (Rendering|SetActorHiddenInGame (Variables|Heart|GetHeartMovingBall) true)
  (Variables|Default|SetFinishedTopPuzzle? false))

(event EventTick
  (params (DeltaSeconds :type Float%20%28single-precision%29))
  (if (Variables|InputAndCollision|GetbWatchingActive)
    (Rendering|SetActorHiddenInGame (Variables|InputAndCollision|GetLetGoNinjaActor) false)
    (if (>= (- (Utilities|Time|GetGameTimeinSeconds) (Variables|InputAndCollision|GetLastInputTime)) 7.0)
      (Variables|Default|SetFinishedTopPuzzle? true)
      (Variables|InputAndCollision|SetbWatchingActive false)
      (Rendering|SetActorHiddenInGame (Variables|Heart|GetHeartMovingBall) false)
      (Rendering|SetActorHiddenInGame (Variables|Default|GetBrainSmokeFire) true)
      (Utilities|FlowControl|DoOnce false
        (:Completed
          (Default|AddNextTwoLayers (Variables|Default|GetDynamicMusicPlayer))
          (Audio|PlaySound2D "/Game/Zaid/sample_confirm_accept02_kofi_by_miraclei-364180.sample_confirm_accept02_kofi_by_miraclei-364180" 1.0 1.0 0.0 0 0))))
    (else
      (Rendering|SetActorHiddenInGame (Variables|InputAndCollision|GetLetGoNinjaActor) true))))

(fn ConstructionScript)