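; One-shot portal trigger that plays a short first-person cutscene and teleports the player to a destination.
; On overlap it disables input and lerps the character into the portal, with each update playing the optional sound and restarting the cutscene.
; A panic or normal timeline drives camera pitch, yaw and exposure on a tagged PostProcessVolume.
; On finish it restores camera control, teleports, picks first or third person, and reapplies saved post-process settings.
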(event OnComponentBeginOverlap(Trigger)
  (params (OverlappedComponent :type Primitive%20Component%20Object%20Reference) (OtherActor :type Actor%20Object%20Reference) (OtherComp :type Primitive%20Component%20Object%20Reference) (OtherBodyIndex :type Integer) (bFromSweep :type Boolean) (SweepResult :type Hit%20Result%20Structure%20%28by%20ref%29))
  (bind _sound (Variables|Default|GetSound))
  (bind _asbp_third_person_character (Utilities|Casting|CastToBP_ThirdPersonCharacter OtherActor))
  (if (not (Variables|Default|GetIsTriggered))
    (Variables|Default|SetIsTriggered true)
    ;[0.05057 0.05089 0.15 0.5] Move the Player Inside the Portal
    (Input|DisableInput _asbp_third_person_character (Game|GetPlayerController 0))
    (bind _lerpamount (Timeline|MoveInsidePortal PlayFromStart)
      (:Update
        (Transformation|SetActorLocation _asbp_third_person_character (Math|Vector|Lerp(Vector) (Transformation|GetActorLocation _asbp_third_person_character) (Variables|Default|GetPortalLocation) _lerpamount) false false)
        ;[0.1817 0.3594 0.1197 0.5] Play Interaction Sound if there is any
        (Utilities|IsValid _sound
          (:Is%20Valid
            (Audio|PlaySound2D _sound (Variables|Default|GetSound%20Volume%20Multiplier) 1.0 0.0 0 0 false))
          (:Is%20Not%20Valid
            _))
        (Default|FPCameraActive _asbp_third_person_character)
        (Variables|/Script/Engine.CameraComponent|SetbUsePawnControlRotation (Variables|/Game/BluePrints/MainCharacter/ThirdPerson/Blueprints/BP_ThirdPersonCharacter.BP_ThirdPersonCharacter_C|GetFP_Camera _asbp_third_person_character) false)
        (bind _outactors (Actor|GetAllActorsOfClasswithTag "/Script/Engine.PostProcessVolume" (Variables|Default|GetCurrentPPTag)))
        (Variables|Default|SetOriginalPPSettings (Variables|/Script/Engine.PostProcessVolume|GetSettings (Utilities|Array|Get(acopy) _outactors)))
        (if (Variables|Default|GetPlayerIsPanicking)
          (bind (_direction _pitchvalue_updown _yawvalue_leftright _ppexposurevalue) (Timeline|PortalCutscenePanic PlayFromStart)
            (:Update
              (Transformation|SetRelativeRotation (Variables|/Game/BluePrints/MainCharacter/ThirdPerson/Blueprints/BP_ThirdPersonCharacter.BP_ThirdPersonCharacter_C|GetFP_Camera _asbp_third_person_character) (Math|Rotator|MakeRotator 0.0 _pitchvalue_updown _yawvalue_leftright) false false)
              (Utilities|Struct|SetmembersinPostProcessSettings (Variables|/Script/Engine.PostProcessVolume|GetSettings (Utilities|Array|Get(acopy) _outactors)) "AEM_Manual" _ppexposurevalue))
            (:Finished
              (Variables|/Script/Engine.CameraComponent|SetbUsePawnControlRotation (Variables|/Game/BluePrints/MainCharacter/ThirdPerson/Blueprints/BP_ThirdPersonCharacter.BP_ThirdPersonCharacter_C|GetFP_Camera _asbp_third_person_character) true :!label _label)
              (Default|TeleportPlayer _asbp_third_person_character (Variables|Default|GetTeleportLocation) (Variables|Default|GetTeleportRotation))
              (if (Variables|Default|GetNextLevelIsFirstPerson)
                (Default|FPCameraActive _asbp_third_person_character)
                (else
                  (Default|TPCameraActive _asbp_third_person_character)))
              (Variables|/Script/Engine.PostProcessVolume|SetSettings (Utilities|Array|Get(acopy) _outactors) (Variables|Default|GetOriginalPPSettings))))
          (else
            (bind (_direction_2 _pitchvalue_updown_2 _yawvalue_leftright_2 _ppexposurevalue_2) (Timeline|PortalCutscene PlayFromStart)
              (:Update
                (Transformation|SetRelativeRotation (Variables|/Game/BluePrints/MainCharacter/ThirdPerson/Blueprints/BP_ThirdPersonCharacter.BP_ThirdPersonCharacter_C|GetFP_Camera _asbp_third_person_character) (Math|Rotator|MakeRotator 0.0 _pitchvalue_updown_2 _yawvalue_leftright_2) false false)
                (Utilities|Struct|SetmembersinPostProcessSettings (Variables|/Script/Engine.PostProcessVolume|GetSettings (Utilities|Array|Get(acopy) _outactors)) "AEM_Manual" _ppexposurevalue_2))
              (:Finished
                (goto _label)))))))))

(fn ConstructionScript)