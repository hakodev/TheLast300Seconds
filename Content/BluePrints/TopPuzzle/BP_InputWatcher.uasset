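; BP_InputWatcher is an idle-watcher actor, filed under TopPuzzle, that flags seven seconds elapsed after something overlaps its sphere.
; Any sphere overlap enables input from player controller 0, stamps the game time and starts watching.
; Tick compares elapsed time to that stamp, then prints an idle message and stops watching.
; No input event refreshes the stamp, so only another overlap restarts the countdown.
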(event OnComponentBeginOverlap(Sphere)
  (params (OverlappedComponent :type Primitive%20Component%20Object%20Reference) (OtherActor :type Actor%20Object%20Reference) (OtherComp :type Primitive%20Component%20Object%20Reference) (OtherBodyIndex :type Integer) (bFromSweep :type Boolean) (SweepResult :type Hit%20Result%20Structure%20%28by%20ref%29))
  (Variables|Default|SetbWatchingActive true)
  (Input|EnableInput (Game|GetPlayerController 0))
  (Variables|Default|SetLastInputTime (Utilities|Time|GetGameTimeinSeconds)))

(event EventTick
  (params (DeltaSeconds :type Float%20%28single-precision%29))
  (if (Variables|Default|GetbWatchingActive)
    (if (>= (- (Utilities|Time|GetGameTimeinSeconds) (Variables|Default|GetLastInputTime)) 7.0)
      (Development|PrintString "HasBeenIdleFor7Seconds")
      (Variables|Default|SetbWatchingActive false))))

(fn ConstructionScript)