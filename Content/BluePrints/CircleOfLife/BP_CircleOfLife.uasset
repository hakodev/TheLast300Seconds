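; Circle of Life puzzle actor, where the player docks the hoverboard at platforms and rotates circles to deliver seven balls.
; Platform overlaps set the dock target and active circle, which Tick yaws with the docked board's rotation.
; Balls reaching matching triggers detach, snap into place, glow and advance PuzzleProgress, updating the human actor's material.
; Ball03 counts twice, reaching the total of eight that sets FinishedLeftPuzzle and adds music layers.
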(event OnComponentBeginOverlap(Platform01_Collision)
  (params (OverlappedComponent :type Primitive%20Component%20Object%20Reference) (OtherActor :type Actor%20Object%20Reference) (OtherComp :type Primitive%20Component%20Object%20Reference) (OtherBodyIndex :type Integer) (bFromSweep :type Boolean) (SweepResult :type Hit%20Result%20Structure%20%28by%20ref%29))
  ;[0.15 0 0.06641 0.5] Platform _ 01
  (if (== OtherActor (Variables|Default|GetHoverBoardReference))
    (Default|SetDockTarget (Variables|Default|GetHoverBoardReference) (Variables|Default|GetPlatform01_Position))
    (Variables|Default|SetActiveCircle (Variables|Default|GetCircle1))))

(event OnComponentEndOverlap(Platform01_Collision)
  (params (OverlappedComponent :type Primitive%20Component%20Object%20Reference) (OtherActor :type Actor%20Object%20Reference) (OtherComp :type Primitive%20Component%20Object%20Reference) (OtherBodyIndex :type Integer))
  ;[0.15 0 0.06641 0.5] Platform _ 01
  (if (== OtherActor (Variables|Default|GetHoverBoardReference))
    (Default|ResetDockingTarget (Variables|Default|GetHoverBoardReference))
    (Variables|Default|SetActiveCircle 0)))

(event OnComponentBeginOverlap(Platform07_Collision)
  (params (OverlappedComponent :type Primitive%20Component%20Object%20Reference) (OtherActor :type Actor%20Object%20Reference) (OtherComp :type Primitive%20Component%20Object%20Reference) (OtherBodyIndex :type Integer) (bFromSweep :type Boolean) (SweepResult :type Hit%20Result%20Structure%20%28by%20ref%29))
  ;[0.15 0.15 0.15 0.5] Platform _ 07
  (if (== OtherActor (Variables|Default|GetHoverBoardReference))
    (Default|SetDockTarget (Variables|Default|GetHoverBoardReference) (Variables|Default|GetPlatform07_Position))
    (Variables|Default|SetActiveCircle (Variables|Default|GetCircle7))))

(event OnComponentEndOverlap(Platform07_Collision)
  (params (OverlappedComponent :type Primitive%20Component%20Object%20Reference) (OtherActor :type Actor%20Object%20Reference) (OtherComp :type Primitive%20Component%20Object%20Reference) (OtherBodyIndex :type Integer))
  ;[0.15 0.15 0.15 0.5] Platform _ 07
  (if (== OtherActor (Variables|Default|GetHoverBoardReference))
    (Default|ResetDockingTarget (Variables|Default|GetHoverBoardReference))
    (Variables|Default|SetActiveCircle 0)))

(event OnComponentBeginOverlap(Platform04_Collision)
  (params (OverlappedComponent :type Primitive%20Component%20Object%20Reference) (OtherActor :type Actor%20Object%20Reference) (OtherComp :type Primitive%20Component%20Object%20Reference) (OtherBodyIndex :type Integer) (bFromSweep :type Boolean) (SweepResult :type Hit%20Result%20Structure%20%28by%20ref%29))
  ;[0.15 0.15 0.15 0.5] Platform _ 04
  (if (== OtherActor (Variables|Default|GetHoverBoardReference))
    (Default|SetDockTarget (Variables|Default|GetHoverBoardReference) (Variables|Default|GetPlatform04_Position))
    (Variables|Default|SetActiveCircle (Variables|Default|GetCircle4))))

(event OnComponentEndOverlap(Platform04_Collision)
  (params (OverlappedComponent :type Primitive%20Component%20Object%20Reference) (OtherActor :type Actor%20Object%20Reference) (OtherComp :type Primitive%20Component%20Object%20Reference) (OtherBodyIndex :type Integer))
  ;[0.15 0.15 0.15 0.5] Platform _ 04
  (if (== OtherActor (Variables|Default|GetHoverBoardReference))
    (Default|ResetDockingTarget (Variables|Default|GetHoverBoardReference))
    (Variables|Default|SetActiveCircle 0)))

(event OnComponentBeginOverlap(Platform02_BallCollision)
  (params (OverlappedComponent :type Primitive%20Component%20Object%20Reference) (OtherActor :type Actor%20Object%20Reference) (OtherComp :type Primitive%20Component%20Object%20Reference) (OtherBodyIndex :type Integer) (bFromSweep :type Boolean) (SweepResult :type Hit%20Result%20Structure%20%28by%20ref%29))
  (if (== OtherComp (Variables|Default|GetBall_01))
    (CallFunction|AttachBalltoPlatform (Variables|Default|GetBall_01) (Variables|Default|GetLocation_BallPosition_01))
    (Utilities|IsValid (Variables|Default|GetHumanActorRef)
      (:Is%20Valid
        (bind _result (Math|Integer|IncrementInt (Variables|Default|GetPuzzleProgress))
          (:%20%20
            (Default|UpdateMaterial (Variables|Default|GetHumanActorRef) (- _result 1))
            (Rendering|Material|SetMaterial (Variables|Default|GetBall_01) 0 "/Game/FluidNinjaLive/Tutorial/Materials/MI_CheckerGlow_Zia2.MI_CheckerGlow_Zia2")
            (Rendering|Material|SetMaterial (Variables|Default|GetPlatform1) 0 "/Game/GabrielContent/RIGHT_PUZZLE/Puzzle_Base.Puzzle_Base")))))))

(event OnComponentBeginOverlap(Platform04_BallCollision)
  (params (OverlappedComponent :type Primitive%20Component%20Object%20Reference) (OtherActor :type Actor%20Object%20Reference) (OtherComp :type Primitive%20Component%20Object%20Reference) (OtherBodyIndex :type Integer) (bFromSweep :type Boolean) (SweepResult :type Hit%20Result%20Structure%20%28by%20ref%29))
  (if (== OtherComp (Variables|Default|GetBall_02))
    (CallFunction|AttachBalltoPlatform (Variables|Default|GetBall_02) (Variables|Default|GetLocation_BallPosition_02))
    (Utilities|IsValid (Variables|Default|GetHumanActorRef)
      (:Is%20Valid
        (bind _result (Math|Integer|IncrementInt (Variables|Default|GetPuzzleProgress))
          (:%20%20
            (Default|UpdateMaterial (Variables|Default|GetHumanActorRef) (- _result 1))
            (Rendering|Material|SetMaterial (Variables|Default|GetBall_02) 0 "/Game/FluidNinjaLive/Tutorial/Materials/MI_CheckerGlow_Zia2.MI_CheckerGlow_Zia2")
            (Rendering|Material|SetMaterial (Variables|Default|GetPlatform2) 0 "/Game/GabrielContent/RIGHT_PUZZLE/Puzzle_Base.Puzzle_Base")))))))

(event OnComponentBeginOverlap(Platform05_BallCollision)
  (params (OverlappedComponent :type Primitive%20Component%20Object%20Reference) (OtherActor :type Actor%20Object%20Reference) (OtherComp :type Primitive%20Component%20Object%20Reference) (OtherBodyIndex :type Integer) (bFromSweep :type Boolean) (SweepResult :type Hit%20Result%20Structure%20%28by%20ref%29))
  (if (== OtherComp (Variables|Default|GetBall_03))
    (CallFunction|AttachBalltoPlatform (Variables|Default|GetBall_03) (Variables|Default|GetLocation_BallPosition_03))
    (Utilities|IsValid (Variables|Default|GetHumanActorRef)
      (:Is%20Valid
        (bind _result (Math|Integer|IncrementInt (Variables|Default|GetPuzzleProgress))
          (:%20%20
            (Default|UpdateMaterial (Variables|Default|GetHumanActorRef) (- _result 1))
            (bind _result_2 (Math|Integer|IncrementInt (Variables|Default|GetPuzzleProgress))
              (:%20%20
                (Default|UpdateMaterial (Variables|Default|GetHumanActorRef) (- _result_2 1))
                (Rendering|Material|SetMaterial (Variables|Default|GetBall_03) 0 "/Game/FluidNinjaLive/Tutorial/Materials/MI_CheckerGlow_Zia2.MI_CheckerGlow_Zia2")
                (Rendering|Material|SetMaterial (Variables|Default|GetPlatform3) 0 "/Game/GabrielContent/RIGHT_PUZZLE/Puzzle_Base.Puzzle_Base")))))))))

(event OnComponentBeginOverlap(Platform01_BallCollision)
  (params (OverlappedComponent :type Primitive%20Component%20Object%20Reference) (OtherActor :type Actor%20Object%20Reference) (OtherComp :type Primitive%20Component%20Object%20Reference) (OtherBodyIndex :type Integer) (bFromSweep :type Boolean) (SweepResult :type Hit%20Result%20Structure%20%28by%20ref%29))
  (if (== OtherComp (Variables|Default|GetBall_04))
    (CallFunction|AttachBalltoPlatform (Variables|Default|GetBall_04) (Variables|Default|GetLocation_BallPosition_04))
    (Utilities|IsValid (Variables|Default|GetHumanActorRef)
      (:Is%20Valid
        (bind _result (Math|Integer|IncrementInt (Variables|Default|GetPuzzleProgress))
          (:%20%20
            (Default|UpdateMaterial (Variables|Default|GetHumanActorRef) (- _result 1))
            (Rendering|Material|SetMaterial (Variables|Default|GetBall_04) 0 "/Game/FluidNinjaLive/Tutorial/Materials/MI_CheckerGlow_Zia2.MI_CheckerGlow_Zia2")
            (Rendering|Material|SetMaterial (Variables|Default|GetPlatform4) 0 "/Game/GabrielContent/RIGHT_PUZZLE/Puzzle_Base.Puzzle_Base")))))))

(event OnComponentBeginOverlap(Platform03_BallCollision)
  (params (OverlappedComponent :type Primitive%20Component%20Object%20Reference) (OtherActor :type Actor%20Object%20Reference) (OtherComp :type Primitive%20Component%20Object%20Reference) (OtherBodyIndex :type Integer) (bFromSweep :type Boolean) (SweepResult :type Hit%20Result%20Structure%20%28by%20ref%29))
  (if (== OtherComp (Variables|Default|GetBall_05))
    (CallFunction|AttachBalltoPlatform (Variables|Default|GetBall_05) (Variables|Default|GetLocation_BallPosition_05))
    (Utilities|IsValid (Variables|Default|GetHumanActorRef)
      (:Is%20Valid
        (bind _result (Math|Integer|IncrementInt (Variables|Default|GetPuzzleProgress))
          (:%20%20
            (Default|UpdateMaterial (Variables|Default|GetHumanActorRef) (- _result 1))
            (Rendering|Material|SetMaterial (Variables|Default|GetBall_05) 0 "/Game/FluidNinjaLive/Tutorial/Materials/MI_CheckerGlow_Zia2.MI_CheckerGlow_Zia2")
            (Rendering|Material|SetMaterial (Variables|Default|GetPlatform6) 0 "/Game/GabrielContent/RIGHT_PUZZLE/Puzzle_Base.Puzzle_Base")))))))

(event OnComponentBeginOverlap(Platform07_BallCollision)
  (params (OverlappedComponent :type Primitive%20Component%20Object%20Reference) (OtherActor :type Actor%20Object%20Reference) (OtherComp :type Primitive%20Component%20Object%20Reference) (OtherBodyIndex :type Integer) (bFromSweep :type Boolean) (SweepResult :type Hit%20Result%20Structure%20%28by%20ref%29))
  (if (== OtherComp (Variables|Default|GetBall_06))
    (CallFunction|AttachBalltoPlatform (Variables|Default|GetBall_06) (Variables|Default|GetLocation_BallPosition_06))
    (Utilities|IsValid (Variables|Default|GetHumanActorRef)
      (:Is%20Valid
        (bind _result (Math|Integer|IncrementInt (Variables|Default|GetPuzzleProgress))
          (:%20%20
            (Default|UpdateMaterial (Variables|Default|GetHumanActorRef) (- _result 1))
            (Rendering|Material|SetMaterial (Variables|Default|GetBall_06) 0 "/Game/FluidNinjaLive/Tutorial/Materials/MI_CheckerGlow_Zia2.MI_CheckerGlow_Zia2")
            (Rendering|Material|SetMaterial (Variables|Default|GetPlatform5) 0 "/Game/GabrielContent/RIGHT_PUZZLE/Puzzle_Base.Puzzle_Base")))))))

(event OnComponentBeginOverlap(Platform02_Collision)
  (params (OverlappedComponent :type Primitive%20Component%20Object%20Reference) (OtherActor :type Actor%20Object%20Reference) (OtherComp :type Primitive%20Component%20Object%20Reference) (OtherBodyIndex :type Integer) (bFromSweep :type Boolean) (SweepResult :type Hit%20Result%20Structure%20%28by%20ref%29))
  ;[0.15 0.15 0.15 0.5] Platform _ 02
  (if (== OtherActor (Variables|Default|GetHoverBoardReference))
    (Default|SetDockTarget (Variables|Default|GetHoverBoardReference) (Variables|Default|GetPlatform02_Position))
    (Variables|Default|SetActiveCircle (Variables|Default|GetCircle2))))

(event OnComponentBeginOverlap(Platform06_BallCollision)
  (params (OverlappedComponent :type Primitive%20Component%20Object%20Reference) (OtherActor :type Actor%20Object%20Reference) (OtherComp :type Primitive%20Component%20Object%20Reference) (OtherBodyIndex :type Integer) (bFromSweep :type Boolean) (SweepResult :type Hit%20Result%20Structure%20%28by%20ref%29))
  (if (== OtherComp (Variables|Default|GetBall_07))
    (CallFunction|AttachBalltoPlatform (Variables|Default|GetBall_07) (Variables|Default|GetLocation_BallPosition_07))
    (Utilities|IsValid (Variables|Default|GetHumanActorRef)
      (:Is%20Valid
        (bind _result (Math|Integer|IncrementInt (Variables|Default|GetPuzzleProgress))
          (:%20%20
            (Default|UpdateMaterial (Variables|Default|GetHumanActorRef) (- _result 1))
            (Rendering|Material|SetMaterial (Variables|Default|GetBall_07) 0 "/Game/FluidNinjaLive/Tutorial/Materials/MI_CheckerGlow_Zia2.MI_CheckerGlow_Zia2")
            (Rendering|Material|SetMaterial (Variables|Default|GetPlatform7) 0 "/Game/GabrielContent/RIGHT_PUZZLE/Puzzle_Base.Puzzle_Base")))))))

(event OnComponentBeginOverlap(HUD_Collision)
  (params (OverlappedComponent :type Primitive%20Component%20Object%20Reference) (OtherActor :type Actor%20Object%20Reference) (OtherComp :type Primitive%20Component%20Object%20Reference) (OtherBodyIndex :type Integer) (bFromSweep :type Boolean) (SweepResult :type Hit%20Result%20Structure%20%28by%20ref%29))
  (if (== OtherActor (Variables|Default|GetHoverBoardReference))
    (bind _asui_hud (Utilities|Casting|CastToUI_HUD (HUD|GetHUD (Game|GetPlayerController 0))))
    (Default|EnableEforPuzzle (Variables|/Game/Zaid/UI_HUD.UI_HUD_C|GetUI_Ref _asui_hud))))

(event OnComponentEndOverlap(Platform02_Collision)
  (params (OverlappedComponent :type Primitive%20Component%20Object%20Reference) (OtherActor :type Actor%20Object%20Reference) (OtherComp :type Primitive%20Component%20Object%20Reference) (OtherBodyIndex :type Integer))
  ;[0.15 0.15 0.15 0.5] Platform _ 02
  (if (== OtherActor (Variables|Default|GetHoverBoardReference))
    (Default|ResetDockingTarget (Variables|Default|GetHoverBoardReference))
    (Variables|Default|SetActiveCircle 0)))

(event OnComponentBeginOverlap(Platform03_Collision)
  (params (OverlappedComponent :type Primitive%20Component%20Object%20Reference) (OtherActor :type Actor%20Object%20Reference) (OtherComp :type Primitive%20Component%20Object%20Reference) (OtherBodyIndex :type Integer) (bFromSweep :type Boolean) (SweepResult :type Hit%20Result%20Structure%20%28by%20ref%29))
  ;[0.15 0.15 0.15 0.5] Platform _ 03
  (if (== OtherActor (Variables|Default|GetHoverBoardReference))
    (Default|SetDockTarget (Variables|Default|GetHoverBoardReference) (Variables|Default|GetPlatform03_Position))
    (Variables|Default|SetActiveCircle (Variables|Default|GetCircle3))))

(event OnComponentEndOverlap(Platform03_Collision)
  (params (OverlappedComponent :type Primitive%20Component%20Object%20Reference) (OtherActor :type Actor%20Object%20Reference) (OtherComp :type Primitive%20Component%20Object%20Reference) (OtherBodyIndex :type Integer))
  ;[0.15 0.15 0.15 0.5] Platform _ 03
  (if (== OtherActor (Variables|Default|GetHoverBoardReference))
    (Default|ResetDockingTarget (Variables|Default|GetHoverBoardReference))
    (Variables|Default|SetActiveCircle 0)))

(event OnComponentBeginOverlap(Platform05_Collision)
  (params (OverlappedComponent :type Primitive%20Component%20Object%20Reference) (OtherActor :type Actor%20Object%20Reference) (OtherComp :type Primitive%20Component%20Object%20Reference) (OtherBodyIndex :type Integer) (bFromSweep :type Boolean) (SweepResult :type Hit%20Result%20Structure%20%28by%20ref%29))
  ;[0.15 0.15 0.15 0.5] Platerform _ 05
  (if (== OtherActor (Variables|Default|GetHoverBoardReference))
    (Default|SetDockTarget (Variables|Default|GetHoverBoardReference) (Variables|Default|GetPlatform05_Position))
    (Variables|Default|SetActiveCircle (Variables|Default|GetCircle5))))

(event OnComponentEndOverlap(Platform05_Collision)
  (params (OverlappedComponent :type Primitive%20Component%20Object%20Reference) (OtherActor :type Actor%20Object%20Reference) (OtherComp :type Primitive%20Component%20Object%20Reference) (OtherBodyIndex :type Integer))
  ;[0.15 0.15 0.15 0.5] Platerform _ 05
  (if (== OtherActor (Variables|Default|GetHoverBoardReference))
    (Default|ResetDockingTarget (Variables|Default|GetHoverBoardReference))
    (Variables|Default|SetActiveCircle 0)))

(event OnComponentBeginOverlap(Platform06_Collision)
  (params (OverlappedComponent :type Primitive%20Component%20Object%20Reference) (OtherActor :type Actor%20Object%20Reference) (OtherComp :type Primitive%20Component%20Object%20Reference) (OtherBodyIndex :type Integer) (bFromSweep :type Boolean) (SweepResult :type Hit%20Result%20Structure%20%28by%20ref%29))
  ;[0.15 0.15 0.15 0.5] Platerform _ 06
  (if (== OtherActor (Variables|Default|GetHoverBoardReference))
    (Default|SetDockTarget (Variables|Default|GetHoverBoardReference) (Variables|Default|GetPlatform06_Position))
    (Variables|Default|SetActiveCircle (Variables|Default|GetCircle6))))

(event OnComponentEndOverlap(Platform06_Collision)
  (params (OverlappedComponent :type Primitive%20Component%20Object%20Reference) (OtherActor :type Actor%20Object%20Reference) (OtherComp :type Primitive%20Component%20Object%20Reference) (OtherBodyIndex :type Integer))
  ;[0.15 0.15 0.15 0.5] Platerform _ 06
  (if (== OtherActor (Variables|Default|GetHoverBoardReference))
    (Default|ResetDockingTarget (Variables|Default|GetHoverBoardReference))
    (Variables|Default|SetActiveCircle 0)))

(event EventBeginPlay
  (Variables|Default|SetFinishedLeftPuzzle%20? false))

(event EventTick
  (params (DeltaSeconds :type Float%20%28single-precision%29))
  (Utilities|FlowControl|Sequence
    (:then_0
      (Utilities|IsValid (Variables|Default|GetHoverBoardReference)
        (:Is%20Valid
          (if (Variables|/Game/BluePrints/HoverBoard/BP-HoverBoardPawn.BP-HoverBoardPawn_C|GetIsDocked (Variables|Default|GetHoverBoardReference))
            (Transformation|SetWorldRotation (Variables|Default|GetActiveCircle) (Math|Rotator|MakeRotator 0.0 0.0 (.Yaw (Math|Rotator|BreakRotator (Math|Rotator|CombineRotators (Math|Rotator|Delta(Rotator) (Transformation|GetActorRotation (Variables|Default|GetHoverBoardReference)) (Variables|/Game/BluePrints/HoverBoard/BP-HoverBoardPawn.BP-HoverBoardPawn_C|GetDockedBoardRotation (Variables|Default|GetHoverBoardReference))) (Variables|/Game/BluePrints/HoverBoard/BP-HoverBoardPawn.BP-HoverBoardPawn_C|GetInitialCircleRotation (Variables|Default|GetHoverBoardReference)))))) false false)))))
    (:then_1
      (if (== (Variables|Default|GetPuzzleProgress) 8)
        (Variables|Default|SetFinishedLeftPuzzle%20? true)
        (Utilities|FlowControl|DoOnce false
          (:Completed
            (Default|AddNextTwoLayers (Variables|Default|GetDynamicMusicPlayer))
            (Audio|PlaySound2D "/Game/Zaid/sample_confirm_accept02_kofi_by_miraclei-364180.sample_confirm_accept02_kofi_by_miraclei-364180" 1.0 1.0 0.0 0 0)))))))

(fn ConstructionScript)

(fn SetCircleMaterial
  (params (IsActiveMaterial :type Boolean))
  (Utilities|IsValid (Variables|Default|GetActiveCircle)
    (:Is%20Valid
      (if IsActiveMaterial
        (Rendering|Material|SetMaterial (Variables|Default|GetActiveCircle) 0 (Variables|Default|GetActiveMaterial))
        (else
          (Rendering|Material|SetMaterial (Variables|Default|GetActiveCircle) 0 (Variables|Default|GetDefaultMaterial)))))))

(fn AttachBalltoPlatform
  (params (Ball :type Static%20Mesh%20Component%20Object%20Reference) (PlatformPosition :type Scene%20Component%20Object%20Reference))
  (Transformation|DetachFromComponent Ball "KeepWorld" "KeepWorld" "KeepWorld" true)
  (Transformation|SetWorldLocation Ball (Transformation|GetWorldLocation PlatformPosition) false false))