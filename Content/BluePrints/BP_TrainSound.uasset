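; BP_TrainSound plays a recurring train sound effect as non-spatial 2D audio.
; From BeginPlay, a self-calling event waits a random interval, then spawns the SFX_MatrixTrain_Cue sound with a slightly randomized pitch multiplier.
; It then waits for the sound's duration multiplied by that pitch value before starting the cycle again, with no stop condition.
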(event Custom|PlayTrainSound
  (Utilities|FlowControl|Delay (Math|Random|RandomFloatinRange 1e+01 3e+01))
  (bind _returnvalue (Math|Random|RandomFloatinRange 0.9 1.1))
  (bind _output_get (Variables|Default|SetPitch%20Multiplier _returnvalue))
  (bind _returnvalue_2 (Audio|SpawnSound2D "/Game/Audio/SFX/SFX_MatrixTrain_Cue.SFX_MatrixTrain_Cue" 1.0 _output_get 0.0 0))
  (Utilities|FlowControl|Delay (* (Variables|/Script/Engine.SoundBase|GetDuration (Variables|/Script/Engine.AudioComponent|GetSound _returnvalue_2)) (Variables|Default|GetPitch%20Multiplier)))
  (CallFunction|PlayTrainSound))

(event EventBeginPlay
  (CallFunction|PlayTrainSound))

(fn ConstructionScript)