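; BP_RightPuzzle is the right-hand tube puzzle, solved when all four tubes reach the ending point.
; Tagged tube-end overlaps toggle each reached flag and tube/pattern materials, though any single hit also sets IsSolved.
; Tick polls the four flags, sets FinishedRightPuzzle, and once adds music layers and plays a confirm sound.
; A separate collision enables the HUD's E for the puzzle when the hoverboard enters.
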(event OnComponentBeginOverlap(EndingPointCollision)
  (params (OverlappedComponent :type Primitive%20Component%20Object%20Reference) (OtherActor :type Actor%20Object%20Reference) (OtherComp :type Primitive%20Component%20Object%20Reference) (OtherBodyIndex :type Integer) (bFromSweep :type Boolean) (SweepResult :type Hit%20Result%20Structure%20%28by%20ref%29))
  (Utilities|FlowControl|Sequence
    (:then_0
      (if (Components|ComponentHasTag OtherComp "TubeEndPointTube01")
        (Variables|Default|SetTube_01_Reached true)
        (Rendering|Material|SetMaterial (Variables|Default|GetTube_01) 0 "/Game/GabrielContent/RIGHT_PUZZLE/Puzzle_Solved.Puzzle_Solved")
        (Rendering|Material|SetMaterial (Variables|Default|Get1_pattern) 0 "/Game/GabrielContent/RIGHT_PUZZLE/Tree_Solved.Tree_Solved")
        (Variables|Default|SetIsSolved? true)))
    (:then_1
      (if (Components|ComponentHasTag OtherComp "TubeEndPointTube02")
        (Variables|Default|SetTube_02_Reached true)
        (Rendering|Material|SetMaterial (Variables|Default|GetTube_02) 0 "/Game/GabrielContent/RIGHT_PUZZLE/Puzzle_Solved.Puzzle_Solved")
        (Rendering|Material|SetMaterial (Variables|Default|Get2_pattern) 0 "/Game/GabrielContent/RIGHT_PUZZLE/Tree_Solved.Tree_Solved")
        (Variables|Default|SetIsSolved? true)))
    (:then_2
      (if (Components|ComponentHasTag OtherComp "TubeEndPointTube03")
        (Variables|Default|SetTube_03_Reached true)
        (Rendering|Material|SetMaterial (Variables|Default|GetTube_03) 0 "/Game/GabrielContent/RIGHT_PUZZLE/Puzzle_Solved.Puzzle_Solved")
        (Rendering|Material|SetMaterial (Variables|Default|Get3_pattern) 0 "/Game/GabrielContent/RIGHT_PUZZLE/Tree_Solved.Tree_Solved")
        (Variables|Default|SetIsSolved? true)))
    (:then_3
      (if (Components|ComponentHasTag OtherComp "TubeEndPointTube04")
        (Variables|Default|SetTube_04_Reached true)
        (Rendering|Material|SetMaterial (Variables|Default|GetTube_0) 0 "/Game/GabrielContent/RIGHT_PUZZLE/Puzzle_Solved.Puzzle_Solved")
        (Rendering|Material|SetMaterial (Variables|Default|Get0_pattern) 0 "/Game/GabrielContent/RIGHT_PUZZLE/Tree_Solved.Tree_Solved")
        (Variables|Default|SetIsSolved? true)))))

(event OnComponentEndOverlap(EndingPointCollision)
  (params (OverlappedComponent :type Primitive%20Component%20Object%20Reference) (OtherActor :type Actor%20Object%20Reference) (OtherComp :type Primitive%20Component%20Object%20Reference) (OtherBodyIndex :type Integer))
  (Utilities|FlowControl|Sequence
    (:then_0
      (if (Components|ComponentHasTag OtherComp "TubeEndPointTube01")
        (Variables|Default|SetTube_01_Reached false)
        (Rendering|Material|SetMaterial (Variables|Default|GetTube_01) 0 "/Game/GabrielContent/RIGHT_PUZZLE/Puzzle_Base.Puzzle_Base")
        (Rendering|Material|SetMaterial (Variables|Default|Get1_pattern) 0 "/Game/GabrielContent/RIGHT_PUZZLE/Tree_Base.Tree_Base")))
    (:then_1
      (if (Components|ComponentHasTag OtherComp "TubeEndPointTube02")
        (Variables|Default|SetTube_02_Reached false)
        (Rendering|Material|SetMaterial (Variables|Default|GetTube_02) 0 "/Game/GabrielContent/RIGHT_PUZZLE/Puzzle_Base.Puzzle_Base")
        (Rendering|Material|SetMaterial (Variables|Default|Get2_pattern) 0 "/Game/GabrielContent/RIGHT_PUZZLE/Tree_Base.Tree_Base")))
    (:then_2
      (if (Components|ComponentHasTag OtherComp "TubeEndPointTube03")
        (Variables|Default|SetTube_03_Reached false)
        (Rendering|Material|SetMaterial (Variables|Default|GetTube_03) 0 "/Game/GabrielContent/RIGHT_PUZZLE/Puzzle_Base.Puzzle_Base")
        (Rendering|Material|SetMaterial (Variables|Default|Get3_pattern) 0 "/Game/GabrielContent/RIGHT_PUZZLE/Tree_Base.Tree_Base")))
    (:then_3
      (if (Components|ComponentHasTag OtherComp "TubeEndPointTube04")
        (Variables|Default|SetTube_04_Reached false)
        (Rendering|Material|SetMaterial (Variables|Default|GetTube_0) 0 "/Game/GabrielContent/RIGHT_PUZZLE/Puzzle_Base.Puzzle_Base")
        (Rendering|Material|SetMaterial (Variables|Default|Get0_pattern) 0 "/Game/GabrielContent/RIGHT_PUZZLE/Tree_Base.Tree_Base")))))

(event OnComponentBeginOverlap(Collision_HUD)
  (params (OverlappedComponent :type Primitive%20Component%20Object%20Reference) (OtherActor :type Actor%20Object%20Reference) (OtherComp :type Primitive%20Component%20Object%20Reference) (OtherBodyIndex :type Integer) (bFromSweep :type Boolean) (SweepResult :type Hit%20Result%20Structure%20%28by%20ref%29))
  (if (== OtherActor (Variables|Default|GetHoverBoard_Ref))
    (bind _asui_hud (Utilities|Casting|CastToUI_HUD (HUD|GetHUD (Game|GetPlayerController 0))))
    (Default|EnableEforPuzzle (Variables|/Game/Zaid/UI_HUD.UI_HUD_C|GetUI_Ref _asui_hud))))

(event EventBeginPlay
  (Variables|Default|SetTube_01_Reached false)
  (Variables|Default|SetTube_02_Reached false)
  (Variables|Default|SetTube_03_Reached false)
  (Variables|Default|SetTube_04_Reached false)
  (Variables|Default|SetIsSolved? false)
  (Variables|Default|SetFinishedRightPuzzle? false))

(event Collision|EventActorBeginOverlap
  (params (OtherActor :type Actor%20Object%20Reference)))

(event EventTick
  (params (DeltaSeconds :type Float%20%28single-precision%29))
  (if (Math|Boolean|ANDBoolean (Variables|Default|GetTube_01_Reached) (Variables|Default|GetTube_02_Reached) (Variables|Default|GetTube_03_Reached) (Variables|Default|GetTube_04_Reached))
    (Variables|Default|SetIsSolved? true)
    (Rendering|Material|SetMaterial (Variables|Default|GetTube_01) 0 "/Game/GabrielContent/RIGHT_PUZZLE/Puzzle_Solved.Puzzle_Solved")
    (Variables|Default|SetFinishedRightPuzzle? true)
    (Utilities|FlowControl|DoOnce false
      (:Completed
        (Default|AddNextTwoLayers (Variables|Default|GetDynamicMusicPlayer))
        (Audio|PlaySound2D "/Game/Zaid/sample_confirm_accept02_kofi_by_miraclei-364180.sample_confirm_accept02_kofi_by_miraclei-364180" 1.0 1.0 0.0 0 0)))))

(fn ConstructionScript)